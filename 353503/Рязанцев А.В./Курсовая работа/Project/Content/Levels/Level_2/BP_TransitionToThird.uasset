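; BP_TransitionToThird is a trigger actor in Level 2 that moves the player on to ThirdLevel once the level is completed.
; It polls BP_SecondGameMode's IsComplited flag every Tick via GetActorOfClass, then latches its own copy and disables its tick.
; When BP_MainCharater begins overlapping its Box after that, it opens ThirdLevel by name.
; Every overlap also prints a debug string, regardless of completion.
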(event OnComponentBeginOverlap(Box)
  (params (OverlappedComponent :type Primitive%20Component%20Object%20Reference) (OtherActor :type Actor%20Object%20Reference) (OtherComp :type Primitive%20Component%20Object%20Reference) (OtherBodyIndex :type Integer) (bFromSweep :type Boolean) (SweepResult :type Hit%20Result%20Structure%20%28by%20ref%29))
  (Development|PrintString "overlap")
  (if (Variables|Default|GetIsComplited)
    (Utilities|Casting|CastToBP_MainCharater OtherActor)
    (Game|OpenLevel(byName) "ThirdLevel")))

(event EventBeginPlay
  (Variables|Default|SetIsComplited false))

(event Collision|EventActorBeginOverlap
  (params (OtherActor :type Actor%20Object%20Reference)))

(event EventTick
  (params (DeltaSeconds :type Float%20%28single-precision%29))
  (bind _returnvalue (Actor|GetActorOfClass "/Game/Levels/Level_2/BP_SecondGameMode.BP_SecondGameMode_C"))
  (if (Variables|/Script/Cursach.BasicGameMode|GetbIsComplited _returnvalue)
    (Variables|Default|SetIsComplited true)
    (Actor|Tick|SetActorTickEnabled false)))

(fn ConstructionScript)