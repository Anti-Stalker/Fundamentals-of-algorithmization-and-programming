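; BP_ThirdGameMode is the Level 3 game mode, which detects when the vase placement puzzle is solved.
; Every Tick it polls all BP_BaseSurface actors, clearing IsComplited and printing a debug dash for each one without its right vase.
; When all surfaces pass, it destroys every BP_BaseVase and disables tick on DefaultSceneRoot only, leaving the actor's own Tick enabled.
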(event EventTick
  (params (DeltaSeconds :type Float%20%28single-precision%29))
  (Variables|Default|SetbIsComplited true)
  (bind _outactors (Actor|GetAllActorsOfClass "/Game/BPs/Control/BP_BaseSurface.BP_BaseSurface_C"))
  (for _array_element _outactors
    (if (not (Variables|/Game/BPs/Control/BP_BaseSurface.BP_BaseSurface_C|GetHasRigthtVase _array_element))
      (Variables|Default|SetbIsComplited false)
      (Development|PrintString "-")))
  (if (Variables|Default|GetbIsComplited)
    (bind _outactors_2 (Actor|GetAllActorsOfClass "/Game/BPs/Objects/BP_BaseVase.BP_BaseVase_C"))
    (Components|Tick|SetComponentTickEnabled (Variables|Default|GetDefaultSceneRoot) false)
    (for _array_element_2 _outactors_2
      (Actor|DestroyActor _array_element_2))))

(fn ConstructionScript)