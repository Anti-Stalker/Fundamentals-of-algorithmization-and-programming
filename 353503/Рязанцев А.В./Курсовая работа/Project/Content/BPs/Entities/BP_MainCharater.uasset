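; Player character that moves on a 64-unit grid with WASD, fights enemies with a picked-up sword, and restarts the level when hit by one.
; Timelines turn and step the actor, sliding it back when the swept move is blocked, with IsMoving gating input.
; E equips an overlapping BP_Sword via BPI_Sword, also done automatically at BeginPlay outside FirstLevel.
; Left click plays the attack, enabling delayed sword-overlap damage that can destroy enemies.
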(event OnComponentBeginOverlap(Sword)
  (params (OverlappedComponent :type Primitive%20Component%20Object%20Reference) (OtherActor :type Actor%20Object%20Reference) (OtherComp :type Primitive%20Component%20Object%20Reference) (OtherBodyIndex :type Integer) (bFromSweep :type Boolean) (SweepResult :type Hit%20Result%20Structure%20%28by%20ref%29))
  (bind _asbp_enemy_char (Utilities|Casting|CastToBP_EnemyChar OtherActor))
  (Utilities|FlowControl|Delay 1.0)
  (if (Variables|Default|GetbIsAtacking)
    (bind _returnvalue (Class|BaseCharacter|Atack 5e+01 _asbp_enemy_char))
    (if (not _returnvalue)
      (Default|Die _asbp_enemy_char)
      (Actor|DestroyActor _asbp_enemy_char))))

(event EventBeginPlay
  (Class|WidgetBlueprintLibrary|SetFocustoGameViewport)
  (Variables|/Script/Engine.PlayerController|SetbShowMouseCursor (Game|GetPlayerController 0) true)
  (bind _returnvalue (Game|GetCurrentLevelName true))
  (if (not (Utilities|Enum|Equal(Enum) _returnvalue "FirstLevel"))
    (for _array_element (Collision|GetOverlappingActors "/Game/BPs/Objects/BP_Sword.BP_Sword_C" :!class /Script/Engine.Actor)
      (if (Utilities|DoesObjectImplementInterface _array_element "/Game/BPs/Interfaces/BPI_Sword.BPI_Sword_C")
        (Class|BPISword|PickUp(Message) _array_element)
        (bind _asbp_sword (Utilities|Casting|CastToBP_Sword _array_element))
        (Components|StaticMesh|SetStaticMesh (Variables|Default|GetSword) (Variables|/Script/Engine.StaticMeshComponent|GetStaticMesh (Variables|/Game/BPs/Objects/BP_Sword.BP_Sword_C|GetItemModel _asbp_sword)))
        (Variables|Default|SetbIsWeapon true)))))

(event Collision|EventHit
  (params (MyComp :type Primitive%20Component%20Object%20Reference) (Other :type Actor%20Object%20Reference) (OtherComp :type Primitive%20Component%20Object%20Reference) (bSelfMoved :type Boolean) (HitLocation :type Vector :default "0, 0, 0") (HitNormal :type Vector :default "0, 0, 0") (NormalImpulse :type Vector :default "0, 0, 0") (Hit :type Hit%20Result%20Structure%20%28by%20ref%29))
  ;[1 1 1] Atack
  (Utilities|Casting|CastToBP_EnemyChar Other)
  (bind _returnvalue (Game|GetCurrentLevelName true))
  (Game|OpenLevel(byName) (Utilities|String|StringToName _returnvalue)))

(event Input|MouseEvents|LeftMouseButton
  (params (Key :type Key%20Structure :default "None"))
  ;[1 1 1] Atack
  (:Pressed
    (if (not (Variables|Default|GetIsMoving))
      (if (Variables|Default|GetbIsWeapon)
        (Variables|Default|SetIsMoving true)
        (Utilities|FlowControl|DoOnce false :!label _label
          (:Completed
            (Variables|Default|SetbIsAtacking true)
            (Components|Animation|PlayAnimation (Variables|Character|GetMesh) "/Game/Assets/Characters/Character_Texture/Standing_Melee_Attack_Horizontal.Standing_Melee_Attack_Horizontal" false)
            (Utilities|FlowControl|Delay 2.0)
            (Components|Animation|PlayAnimation (Variables|Character|GetMesh) "/Game/Assets/Characters/Character_Texture/Standing_W_Briefcase_Idle.Standing_W_Briefcase_Idle" false)
            (Variables|Default|SetIsMoving false)
            (Variables|Default|SetbIsAtacking false)
            (goto _label Reset)))))))

(event Input|KeyboardEvents|D
  (params (Key :type Key%20Structure :default "None"))
  ;[1 1 1] Move Right
  (:Pressed
    (if (not (Variables|Default|GetIsMoving))
      (Variables|Default|SetRotation (Transformation|GetActorRotation))
      (Variables|Default|SetIsMoving true)
      (bind _movement (Timeline|Timeline_8 PlayFromStart)
        (:Update
          (Transformation|SetActorRotation (Math|Rotator|Lerp(Rotator) (Variables|Default|GetRotation) (Math|Rotator|MakeRotator (.roll (Variables|Default|GetRotation)) (.pitch (Variables|Default|GetRotation)) 0.0) _movement true)))
        (:Finished
          (Variables|Default|SetPlayer%20Pos (Transformation|GetActorLocation))
          (bind _movement_2 (Timeline|Timeline PlayFromStart)
            (:Update
              (bind _returnvalue (Transformation|SetActorLocation (Math|Vector|Lerp(Vector) (Variables|Default|GetPlayer%20Pos) (+ (Variables|Default|GetPlayer%20Pos) "64.000000,0.000000,0.000000") _movement_2) true false)))
            (:Finished
              (Variables|Default|SetIsMoving false)
              (if (not _returnvalue)
                (Variables|Default|SetPos (Transformation|GetActorLocation))
                (Variables|Default|SetIsMoving true)
                (bind _movement_3 (Timeline|Timeline_0 PlayFromStart)
                  (:Update
                    (Transformation|SetActorLocation (Math|Vector|Lerp(Vector) (Variables|Default|GetPos) (Variables|Default|GetPlayer%20Pos) _movement_3) true false))
                  (:Finished
                    (Variables|Default|SetIsMoving false)))))))))))

(event Input|KeyboardEvents|E
  (params (Key :type Key%20Structure :default "None"))
  (:Pressed
    (for _array_element (Collision|GetOverlappingActors "/Game/BPs/Objects/BP_Sword.BP_Sword_C" :!class /Script/Engine.Actor)
      (if (Utilities|DoesObjectImplementInterface _array_element "/Game/BPs/Interfaces/BPI_Sword.BPI_Sword_C")
        (Class|BPISword|PickUp(Message) _array_element)
        (bind _asbp_sword (Utilities|Casting|CastToBP_Sword _array_element))
        (Components|StaticMesh|SetStaticMesh (Variables|Default|GetSword) (Variables|/Script/Engine.StaticMeshComponent|GetStaticMesh (Variables|/Game/BPs/Objects/BP_Sword.BP_Sword_C|GetItemModel _asbp_sword)))
        (Variables|Default|SetbIsWeapon true)))))

(event Input|KeyboardEvents|Backspace
  (params (Key :type Key%20Structure :default "None"))
  (:Pressed
    (Development|PrintString (Utilities|String|ToString(Boolean) (Variables|Default|GetbIsKey)))))

(event Input|KeyboardEvents|S
  (params (Key :type Key%20Structure :default "None"))
  ;[1 1 1] Move down
  (:Pressed
    (if (not (Variables|Default|GetIsMoving))
      (Variables|Default|SetRotation (Transformation|GetActorRotation))
      (Variables|Default|SetIsMoving true)
      (bind _movement (Timeline|Timeline_10 PlayFromStart)
        (:Update
          (Transformation|SetActorRotation (Math|Rotator|Lerp(Rotator) (Variables|Default|GetRotation) (Math|Rotator|MakeRotator (.roll (Variables|Default|GetRotation)) (.pitch (Variables|Default|GetRotation)) 9e+01) _movement true)))
        (:Finished
          (Variables|Default|SetPlayer%20Pos (Transformation|GetActorLocation))
          (bind _movement_2 (Timeline|Timeline_1 PlayFromStart)
            (:Update
              (bind _returnvalue (Transformation|SetActorLocation (Math|Vector|Lerp(Vector) (Variables|Default|GetPlayer%20Pos) (+ (Variables|Default|GetPlayer%20Pos) "0.000000,64.000000,0.000000") _movement_2) true false)))
            (:Finished
              (Variables|Default|SetIsMoving false)
              (if (not _returnvalue)
                (Variables|Default|SetPos (Transformation|GetActorLocation))
                (Variables|Default|SetIsMoving true)
                (bind _movement_3 (Timeline|Timeline_2 PlayFromStart)
                  (:Update
                    (Transformation|SetActorLocation (Math|Vector|Lerp(Vector) (Variables|Default|GetPos) (Variables|Default|GetPlayer%20Pos) _movement_3) true false))
                  (:Finished
                    (Variables|Default|SetIsMoving false)))))))))))

(event Input|KeyboardEvents|A
  (params (Key :type Key%20Structure :default "None"))
  ;[1 1 1] Move Left
  (:Pressed
    (if (not (Variables|Default|GetIsMoving))
      (Variables|Default|SetRotation (Transformation|GetActorRotation))
      (Variables|Default|SetIsMoving true)
      (bind _movement (Timeline|Timeline_9 PlayFromStart)
        (:Update
          (Transformation|SetActorRotation (Math|Rotator|Lerp(Rotator) (Variables|Default|GetRotation) (Math|Rotator|MakeRotator (.roll (Variables|Default|GetRotation)) (.pitch (Variables|Default|GetRotation)) 1.8e+02) _movement true)))
        (:Finished
          (Variables|Default|SetPlayer%20Pos (Transformation|GetActorLocation))
          (bind _movement_2 (Timeline|Timeline_3 PlayFromStart)
            (:Update
              (bind _returnvalue (Transformation|SetActorLocation (Math|Vector|Lerp(Vector) (Variables|Default|GetPlayer%20Pos) (- (Variables|Default|GetPlayer%20Pos) "64.000000,0.000000,0.000000") _movement_2) true false)))
            (:Finished
              (Variables|Default|SetIsMoving false)
              (if (not _returnvalue)
                (Variables|Default|SetPos (Transformation|GetActorLocation))
                (Variables|Default|SetIsMoving true)
                (bind _movement_3 (Timeline|Timeline_4 PlayFromStart)
                  (:Update
                    (Transformation|SetActorLocation (Math|Vector|Lerp(Vector) (Variables|Default|GetPos) (Variables|Default|GetPlayer%20Pos) _movement_3) true false))
                  (:Finished
                    (Variables|Default|SetIsMoving false)))))))))))

(event Input|KeyboardEvents|W
  (params (Key :type Key%20Structure :default "None"))
  ;[1 1 1] Move Up
  (:Pressed
    (if (not (Variables|Default|GetIsMoving))
      (Variables|Default|SetIsMoving true)
      (Variables|Default|SetRotation (Transformation|GetActorRotation))
      (bind _movement (Timeline|Timeline_7 PlayFromStart)
        (:Update
          (Transformation|SetActorRotation (Math|Rotator|Lerp(Rotator) (Variables|Default|GetRotation) (Math|Rotator|MakeRotator (.roll (Variables|Default|GetRotation)) (.pitch (Variables|Default|GetRotation)) -9e+01) _movement true)))
        (:Finished
          (Variables|Default|SetPlayer%20Pos (Transformation|GetActorLocation))
          (bind _movement_2 (Timeline|Timeline_5 PlayFromStart)
            (:Update
              (bind _returnvalue (Transformation|SetActorLocation (Math|Vector|Lerp(Vector) (Variables|Default|GetPlayer%20Pos) (- (Variables|Default|GetPlayer%20Pos) "0.000000,64.000000,0.000000") _movement_2) true false)))
            (:Finished
              (Variables|Default|SetIsMoving false)
              (if (not _returnvalue)
                (Variables|Default|SetPos (Transformation|GetActorLocation))
                (Variables|Default|SetIsMoving true)
                (bind _movement_3 (Timeline|Timeline_6 PlayFromStart)
                  (:Update
                    (Transformation|SetActorLocation (Math|Vector|Lerp(Vector) (Variables|Default|GetPos) (Variables|Default|GetPlayer%20Pos) _movement_3) true false))
                  (:Finished
                    (Variables|Default|SetIsMoving false)))))))))))

(fn ConstructionScript)