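; Enemy character Blueprint for a zombie that moves, attacks and dies, with a level matrix chosen by level name.
; BeginPlay sets up that matrix, converts its world location and loops the walk animation, while Tick calls Action every frame.
; ToMove calls Move, then uses a timeline to lerp the actor to EnemyPos with sweep.
; Death plays an animation and, in FirstLevel, teleports the red vase to EnemyPos.
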(event EventBeginPlay
  (bind _returnvalue (Game|GetCurrentLevelName true))
  (Development|PrintString "Hello")
  (Class|EnemyCharacter|SetLevelMatrix _returnvalue)
  (Class|EnemyCharacter|ConvertEnemyLocation (Transformation|GetActorLocation))
  (Components|Animation|PlayAnimation (Variables|Character|GetMesh) "/Game/Assets/Characters/Enemy_Character/Zombie_Walk_1_.Zombie_Walk_1_" true))

(event EventDie
  (Components|Animation|PlayAnimation (Variables|Character|GetMesh) "/Game/Assets/Characters/Character_Texture/Standing_Death_Forward_01.Standing_Death_Forward_01" false)
  (bind _returnvalue (Game|GetCurrentLevelName true))
  (if (Utilities|Enum|Equal(Enum) _returnvalue "FirstLevel")
    (bind _returnvalue_2 (Actor|GetActorOfClass "/Game/BPs/Objects/BP_RedVase.BP_RedVase_C"))
    (Transformation|SetActorLocation _returnvalue_2 (Variables|Default|GetEnemyPos) false true)))

(event EventTick
  (params (DeltaSeconds :type Float%20%28single-precision%29))
  (Class|EnemyCharacter|Action))

(event EventToMove
  (Variables|Default|SetStart (Variables|Default|GetEnemyPos))
  (Class|EnemyCharacter|Move)
  (bind _alpha (Timeline|Walk PlayFromStart)
    (:Update
      (Transformation|SetActorLocation (Math|Vector|Lerp(Vector) (Variables|Default|GetStart) (Variables|Default|GetEnemyPos) _alpha) true false))))

(event EventToAtack
  (Components|Animation|PlayAnimation (Variables|Character|GetMesh) "/Game/Assets/Characters/Enemy_Character/Zombie_Attack.Zombie_Attack" false))

(fn ConstructionScript)