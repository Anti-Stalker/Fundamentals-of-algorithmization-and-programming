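; BP_BaseSurface is a surface that holds one vase and tracks whether it is the needed color.
; Place spawns the given class at half scale and fixed height when empty.
; RightBox flags an overlapping BP_BaseVase and compares its Color to NeededVase, while the character entering TakeBox clears both vase flags.
; PlaceBox and TakeBox toggle IsOverlaped with opposite polarity; IsRight is an unfinished stub.
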(event OnComponentBeginOverlap(TakeBox)
  (params (OverlappedComponent :type Primitive%20Component%20Object%20Reference) (OtherActor :type Actor%20Object%20Reference) (OtherComp :type Primitive%20Component%20Object%20Reference) (OtherBodyIndex :type Integer) (bFromSweep :type Boolean) (SweepResult :type Hit%20Result%20Structure%20%28by%20ref%29))
  (Utilities|Casting|CastToBP_MainCharater OtherActor)
  (Variables|Default|SetHas%20Vase false)
  (Variables|Default|SetHasRigthtVase false)
  (Variables|Default|SetIsOverlaped false))

(event OnComponentBeginOverlap(RightBox)
  (params (OverlappedComponent :type Primitive%20Component%20Object%20Reference) (OtherActor :type Actor%20Object%20Reference) (OtherComp :type Primitive%20Component%20Object%20Reference) (OtherBodyIndex :type Integer) (bFromSweep :type Boolean) (SweepResult :type Hit%20Result%20Structure%20%28by%20ref%29))
  (bind _asbp_base_vase (Utilities|Casting|CastToBP_BaseVase OtherActor))
  (Variables|Default|SetHas%20Vase true)
  (if (Utilities|Enum|Equal(Enum) (Variables|/Game/BPs/Objects/BP_BaseVase.BP_BaseVase_C|GetColor _asbp_base_vase) (Variables|Default|GetNeededVase))
    (Variables|Default|SetHasRigthtVase true)))

(event OnComponentBeginOverlap(PlaceBox)
  (params (OverlappedComponent :type Primitive%20Component%20Object%20Reference) (OtherActor :type Actor%20Object%20Reference) (OtherComp :type Primitive%20Component%20Object%20Reference) (OtherBodyIndex :type Integer) (bFromSweep :type Boolean) (SweepResult :type Hit%20Result%20Structure%20%28by%20ref%29))
  (Utilities|Casting|CastToBP_MainCharater OtherActor)
  (Variables|Default|SetIsOverlaped true)
  (Development|PrintString (Utilities|GetObjectName OverlappedComponent)))

(event OnComponentEndOverlap(PlaceBox)
  (params (OverlappedComponent :type Primitive%20Component%20Object%20Reference) (OtherActor :type Actor%20Object%20Reference) (OtherComp :type Primitive%20Component%20Object%20Reference) (OtherBodyIndex :type Integer))
  (Utilities|Casting|CastToBP_MainCharater OtherActor)
  (Variables|Default|SetIsOverlaped false))

(event OnComponentEndOverlap(TakeBox)
  (params (OverlappedComponent :type Primitive%20Component%20Object%20Reference) (OtherActor :type Actor%20Object%20Reference) (OtherComp :type Primitive%20Component%20Object%20Reference) (OtherBodyIndex :type Integer))
  (Utilities|Casting|CastToBP_MainCharater OtherActor)
  (Variables|Default|SetIsOverlaped true))

(event EventPlace
  (params (ObjectToSpawn :type Actor%20Class%20Reference))
  (bind _returnvalue (Transformation|GetActorTransform))
  (if (not (Variables|Default|GetHas%20Vase))
    (Game|SpawnActorfromClass ObjectToSpawn (Math|Transform|MakeTransform (Math|Vector|MakeVector (.x (.location _returnvalue)) (.y (.location _returnvalue)) 5e+01) (.rotation _returnvalue) "0.500000,0.500000,0.500000") "Undefined" "MultiplyWithRoot" 0 0)
    (Variables|Default|SetHas%20Vase true)))

(fn ConstructionScript)

(fn IsRight
  (params (Name :type String)))