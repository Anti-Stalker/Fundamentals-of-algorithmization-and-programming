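; BP_Door is a door actor in the 2D game folder that swings when a BP_MainCharater carrying a key overlaps it.
; It checks the character's key flag, then snaps its yaw 90 degrees and offsets its Y position, choosing the direction by whether its roll exceeds 90.
; IsOpened is set only in the roll-above-90 branch and never checked, so each qualifying overlap moves the door again.
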(event EventBeginPlay)

(event EventTick
  (params (DeltaSeconds :type Float%20%28single-precision%29)))

(event Collision|EventActorBeginOverlap
  (params (OtherActor :type Actor%20Object%20Reference))
  (bind _returnvalue (Transformation|GetActorLocation))
  (bind _returnvalue_2 (Transformation|GetActorLocation))
  (bind _asbp_main_charater (Utilities|Casting|CastToBP_MainCharater OtherActor))
  (bind _output_get (Variables|Default|SetRotation (Transformation|GetActorRotation)))
  (bind _returnvalue_3 (Class|MainCharacter|GetIsKey _asbp_main_charater))
  (if _returnvalue_3
    (if (> (.roll _output_get) 9e+01)
      (Transformation|SetActorRotation (Math|Rotator|MakeRotator (.roll (Variables|Default|GetRotation)) (.pitch (Variables|Default|GetRotation)) (- (.yaw (Variables|Default|GetRotation)) 9e+01)))
      (Transformation|SetActorLocation (Math|Vector|MakeVector (.x _returnvalue_2) (+ (.y _returnvalue_2) 15.0) 0.0) false true)
      (Variables|Default|SetIsOpened true)
      (else
        (Transformation|SetActorRotation (Math|Rotator|MakeRotator (.roll (Variables|Default|GetRotation)) (.pitch (Variables|Default|GetRotation)) (+ (.yaw (Variables|Default|GetRotation)) 9e+01)))
        (Transformation|SetActorLocation (Math|Vector|MakeVector (.x _returnvalue) (- (.y _returnvalue) 15.0) 0.0) false true)))))

(fn ConstructionScript)