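; BP_EnemyPawn is an enemy combatant in a turn-based card game, with HP, deck and hand settings loaded from an encounter struct.
; Setup caches the player and Enemy_AI controller and configures a health bar widget.
; Clicking the pawn plays the player's selected card on it if target and AP checks pass, then updates health or reports death to the game mode.
; PlayTurn delegates enemy actions to the AI.
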(event Custom|PlayTurn
  (Variables|Default|SetAPcurrent 99)
  (Class|CardPawn|StartTurn)
  (Default|EventonMyTurn (Variables|Default|GetAI))
  (Development|PrintString "REVENGE!")
  (Class|CardPawn|EndTurn))

(event Custom|Die
  (bind _asbp_karcianka_game_mode_base (Utilities|Casting|CastToBP_KarciankaGameModeBase (Game|GetGameMode)))
  (Default|EnemyDies _asbp_karcianka_game_mode_base self)
  (Actor|DestroyActor))

(event Custom|Setup
  (bind _asbp_player (Utilities|Casting|CastToBP_Player (Game|Player|GetPlayerPawn 0)))
  (Variables|Default|SetPlayer _asbp_player)
  (bind _asprogress_bar_widget (Utilities|Casting|CastToProgressBar_Widget (UserInterface|GetWidget (Variables|Default|GetWidget))))
  (Class|CardPawn|SetProgressBar (Variables|/Game/ProgressBar_Widget.ProgressBar_Widget_C|GetHealthBar _asprogress_bar_widget))
  (Variables|Default|SetHPText (Variables|/Game/ProgressBar_Widget.ProgressBar_Widget_C|GetHPTextBlock _asprogress_bar_widget))
  (Class|CardPawn|UpdateHealthBar)
  (bind _returnvalue (Class|CardPawn|GetProgressBar))
  (Class|ProgressBar|SetFillColorandOpacity _returnvalue "(R=0.817708,G=0.000000,B=0.000000,A=1.000000)")
  (bind _asenemy_ai (Utilities|Casting|CastToEnemy_AI (Pawn|GetController)))
  (Variables|Default|SetAI _asenemy_ai))

(event Custom|Setup%20Values%20from%20Struct
  (params (Enemy%20Encounter :type Enemy%20Encounter%20Structure))
  (bind (_hp _deck _handsize _drawncards) (Utilities|Struct|BreakEnemyEncounter Enemy%20Encounter))
  (bind _output_get (Variables|Default|SetmaxHP _hp))
  (Variables|Default|Sethp _output_get)
  (Variables|Default|SetDeck _deck)
  (Variables|Default|SetHandSize _handsize)
  (Variables|Default|SetDrawnCards _drawncards))

(event MouseInput|EventActorOnClicked
  (params (ButtonPressed :type Key%20Structure :default "None"))
  (Development|PrintString "Clicked")
  (Utilities|IsValid (Variables|Default|GetHandHandler)
    (:Is%20Valid
      _)
    (:Is%20Not%20Valid
      (bind _asbp_player (Utilities|Casting|CastToBP_Player (Game|Player|GetPlayerPawn 0)))
      (Variables|Default|SetHandHandler (Variables|/Game/BP_Player.BP_Player_C|GetHand%20Handler _asbp_player))))
  (Utilities|IsValid (Variables|/Game/BP_HandHandler.BP_HandHandler_C|GetSelected (Variables|Default|GetHandHandler))
    (:Is%20Valid
      (bind _returnvalue (Class|Card|CanbeUsedon (Variables|/Game/BP_HandHandler.BP_HandHandler_C|GetSelected (Variables|Default|GetHandHandler)) "enemy"))
      (if _returnvalue
        (bind _returnvalue_2 (Class|CardPawn|EnoughAPtoPlay (Variables|Default|GetPlayer) (Variables|/Game/BP_HandHandler.BP_HandHandler_C|GetSelected (Variables|Default|GetHandHandler))))
        (if _returnvalue_2
          (Class|CardPawn|Play (Variables|Default|GetPlayer) (Variables|/Game/BP_HandHandler.BP_HandHandler_C|GetSelected (Variables|Default|GetHandHandler)) self)
          (Default|DiscardCard (Variables|Default|GetHandHandler) (Variables|/Game/BP_HandHandler.BP_HandHandler_C|GetSelected (Variables|Default|GetHandHandler)))
          (Development|PrintString "OH NO! A CARD HAS BEEN USED ON ME!")
          (bind _returnvalue_3 (Class|CardPawn|GetHP))
          (if (<= _returnvalue_3 0)
            (CallFunction|Die)
            (else
              (Class|CardPawn|UpdateHealthBar)))
          (else
            (Development|PrintString "Not  enough AP to play")))
        (else
          (Development|PrintString "Card cannot be used on enemy"))))
    (:Is%20Not%20Valid
      (Development|PrintString "Selected card not valid"))))

(fn ConstructionScript)